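; RobotControllerBP is the controller that turns player input into driving and weapon commands for the possessed WheeledRobotPawn.
; On BeginPlay, the local controller adds the VehicleControls Enhanced Input mapping context.
; The EnableWeaponIA action calls the pawn's weapon toggle handler.
; Throttle, brake, steering and handbrake use legacy axis and action events, passed straight to the pawn's vehicle movement component.
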(event Input|EnhancedActionEvents|EnhancedInputActionEnableWeaponIA
  (params (ActionValue :type Boolean) (ElapsedSeconds :type Float%20%28double-precision%29) (TriggeredSeconds :type Float%20%28double-precision%29) (InputAction :type Input%20Action%20Object%20Reference :default "/Game/Blueprints/Input/EnableWeaponIA.EnableWeaponIA"))
  (:Started
    (Class|WheeledRobotPawn|HandleToggleWeaponInput (.AsWheeled%20Robot%20Pawn (Utilities|Casting|CastToWheeledRobotPawn (Pawn|GetControlledPawn))))))

(event EventBeginPlay
  (if (Pawn|IsLocalController)
    (Input|AddMappingContext (PlayerController|LocalPlayerSubsystems|GetEnhancedInputLocalPlayerSubsystem self) "/Game/Blueprints/Input/VehicleControls.VehicleControls" 0 "(bIgnoreAllPressedKeysUntilRelease=True,bForceImmediately=False,bNotifyUserSettings=False)")))

(event Input|ActionEvents|InputActionHandbrake
  (params (Key :type Key%20Structure :default "None"))
  (bind _returnvalue (Pawn|GetControlledPawn))
  (:Pressed
    (bind _aswheeled_robot_pawn (Utilities|Casting|CastToWheeledRobotPawn _returnvalue))
    (Class|ChaosVehicleMovementComponent|SetHandbrakeInput (Variables|/Script/ChaosVehicles.WheeledVehiclePawn|GetVehicleMovementComponent _aswheeled_robot_pawn) true))
  (:Released
    (bind _aswheeled_robot_pawn_2 (Utilities|Casting|CastToWheeledRobotPawn _returnvalue))
    (Class|ChaosVehicleMovementComponent|SetHandbrakeInput (Variables|/Script/ChaosVehicles.WheeledVehiclePawn|GetVehicleMovementComponent _aswheeled_robot_pawn_2) false)))

(event Input|AxisEvents|InputAxisThrottle
  (params (AxisValue :type Float%20%28single-precision%29))
  (bind _aswheeled_robot_pawn (Utilities|Casting|CastToWheeledRobotPawn (Pawn|GetControlledPawn)))
  (Class|ChaosVehicleMovementComponent|SetThrottleInput (Variables|/Script/ChaosVehicles.WheeledVehiclePawn|GetVehicleMovementComponent _aswheeled_robot_pawn) AxisValue))

(event Input|AxisEvents|InputAxisBrake
  (params (AxisValue :type Float%20%28single-precision%29))
  (bind _aswheeled_robot_pawn (Utilities|Casting|CastToWheeledRobotPawn (Pawn|GetControlledPawn)))
  (Class|ChaosVehicleMovementComponent|SetBrakeInput (Variables|/Script/ChaosVehicles.WheeledVehiclePawn|GetVehicleMovementComponent _aswheeled_robot_pawn) AxisValue))

(event Input|AxisEvents|InputAxisSteering
  (params (AxisValue :type Float%20%28single-precision%29))
  (bind _aswheeled_robot_pawn (Utilities|Casting|CastToWheeledRobotPawn (Pawn|GetControlledPawn)))
  (Class|ChaosVehicleMovementComponent|SetSteeringInput (Variables|/Script/ChaosVehicles.WheeledVehiclePawn|GetVehicleMovementComponent _aswheeled_robot_pawn) AxisValue))

(fn ConstructionScript)