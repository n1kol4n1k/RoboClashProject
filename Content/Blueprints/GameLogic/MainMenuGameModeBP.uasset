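; Main menu game mode that presents a choice of three robots (Razor, Reaper, Turtle), highlighting the selected one with a spotlight.
; On BeginPlay it shows the MainMenuBP widget, caches each robot's skeletal mesh and spotlight actors by tag, and hides all lights.
; SelectRobot passes the tag to the widget as the robot name and shows only that robot's light.
; The cached meshes are not used in this graph.
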(event Custom|SelectRobot
  (params (Tag :type Name))
  (bind _razorlight (Variables|Default|GetRazorLight))
  (bind _reaperlight (Variables|Default|GetReaperLight))
  (bind _turtlelight (Variables|Default|GetTurtleLight))
  (bind _rootcomponent (Variables|/Script/Engine.Actor|GetRootComponent _razorlight))
  (bind _rootcomponent_2 (Variables|/Script/Engine.Actor|GetRootComponent _reaperlight))
  (bind _rootcomponent_3 (Variables|/Script/Engine.Actor|GetRootComponent _turtlelight))
  (Default|SetRobotName (Variables|Default|GetMainMenu) Tag)
  (switch name Tag
    (:Razor
      (Rendering|SetVisibility _rootcomponent true false)
      (Rendering|SetVisibility _rootcomponent_2 false false)
      (Rendering|SetVisibility _rootcomponent_3 false false))
    (:Reaper
      (Rendering|SetVisibility _rootcomponent_2 true false)
      (Rendering|SetVisibility _rootcomponent false false)
      (Rendering|SetVisibility _rootcomponent_3 false false))
    (:Turtle
      (Rendering|SetVisibility _rootcomponent_3 true false)
      (Rendering|SetVisibility _rootcomponent false false)
      (Rendering|SetVisibility _rootcomponent_2 false false))))

(event EventBeginPlay
  (bind _returnvalue (UserInterface|CreateWidget "/Game/Blueprints/UI/MainMenuBP.MainMenuBP_C" (Game|GetPlayerController 0)))
  (Variables|Default|SetMainMenu _returnvalue)
  (UserInterface|Viewport|AddtoViewport _returnvalue 0)
  (bind _outactors (Actor|GetAllActorsOfClasswithTag "/Script/Engine.SkeletalMeshActor" "Razor"))
  (Variables|Default|SetRazorMesh (Utilities|Array|Get(acopy) _outactors))
  (bind _outactors_2 (Actor|GetAllActorsOfClasswithTag "/Script/Engine.SpotLight" "Razor"))
  (Variables|Default|SetRazorLight (Utilities|Array|Get(acopy) _outactors_2))
  (bind _outactors_3 (Actor|GetAllActorsOfClasswithTag "/Script/Engine.SkeletalMeshActor" "Reaper"))
  (Variables|Default|SetReaperMesh (Utilities|Array|Get(acopy) _outactors_3))
  (bind _outactors_4 (Actor|GetAllActorsOfClasswithTag "/Script/Engine.SpotLight" "Reaper"))
  (Variables|Default|SetReaperLight (Utilities|Array|Get(acopy) _outactors_4))
  (bind _outactors_5 (Actor|GetAllActorsOfClasswithTag "/Script/Engine.SkeletalMeshActor" "Turtle"))
  (Variables|Default|SetTurtleMesh (Utilities|Array|Get(acopy) _outactors_5))
  (bind _outactors_6 (Actor|GetAllActorsOfClasswithTag "/Script/Engine.SpotLight" "Turtle"))
  (Variables|Default|SetTurtleLight (Utilities|Array|Get(acopy) _outactors_6))
  (Rendering|SetVisibility (Variables|/Script/Engine.Actor|GetRootComponent (Variables|Default|GetRazorLight)) false false)
  (Rendering|SetVisibility (Variables|/Script/Engine.Actor|GetRootComponent (Variables|Default|GetReaperLight)) false false)
  (Rendering|SetVisibility (Variables|/Script/Engine.Actor|GetRootComponent (Variables|Default|GetTurtleLight)) false false))

(fn ConstructionScript)